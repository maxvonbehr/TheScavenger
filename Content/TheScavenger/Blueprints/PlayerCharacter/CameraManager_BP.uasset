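; Player camera manager for the Scavenger character that drives first-person aim-down-sights view and look sway.
; BlueprintUpdateCamera uses control rotation, while ADSCameraAlpha narrows FOV and blends location from the player camera to behind the weapon's RearSight socket.
; The sight-side point is offset along the socket's forward axis by a third of the projected camera-to-sight distance.
; Each tick, SightOffset builds decaying sway from mouse look, added to location in view space.
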(event `self.ReceiveTick`
  (params (DeltaSeconds :type "Float (single-precision)"))
  (`self.SightOffset`))

(event `SightOffset`
  (bind _playerref (`self.PlayerRef`))
  (`/Engine/EditorBlueprintResources/StandardMacros.IsValid` (`self.PlayerRef`)
    (:`Is Valid`
      (set `self.SwayOffset` (`KismetMathLibrary.VInterpTo` (`self.SwayOffset`) (0.0 0.0 0.0) (`GameplayStatics.GetWorldDeltaSeconds`) 8.0))
      (set `self.SwayOffset` (`KismetMathLibrary.VInterpTo` (`self.SwayOffset`) (+ (`self.SwayOffset`) (`KismetMathLibrary.MakeVector` 0.0 (* (`/Game/TheScavenger/Blueprints/PlayerCharacter/Scavenger_Character_BP.MouseLookHorizontal` _playerref) (`self.YawIntensity`)) (* (`/Game/TheScavenger/Blueprints/PlayerCharacter/Scavenger_Character_BP.MouseLookVertical` _playerref) (`self.PitchIntensity`)))) (`GameplayStatics.GetWorldDeltaSeconds`) 5.0)))))

(fn `BlueprintUpdateCamera`
  (params (CameraTarget :type "Actor Object Reference"))
  (returns (NewCameraLocation :type "Vector Structure") (NewCameraRotation :type "Rotator Structure") (NewCameraFOV :type "Float (double-precision)") (ReturnValue :type Boolean))
  (bind _playerref (`self.PlayerRef`))
  (bind _adscameraalpha (`/Game/TheScavenger/Blueprints/PlayerCharacter/Scavenger_Character_BP.ADSCameraAlpha` _playerref))
  (bind (_returnvalue_location _returnvalue_rotation) (`KismetMathLibrary.BreakTransform` (`SceneComponent.GetSocketTransform` (`/Game/TheScavenger/Blueprints/PlayerCharacter/Scavenger_Character_BP.WeaponInHandSM` _playerref) "RearSight" "RTS_World")))
  (bind _returnvalue (`SceneComponent.K2_GetComponentLocation` (`/Game/TheScavenger/Blueprints/PlayerCharacter/Scavenger_Character_BP.PlayerCamera` _playerref)))
  (bind _returnvalue_2 (- _returnvalue_location _returnvalue))
  (bind _returnvalue_3 (`KismetMathLibrary.GetForwardVector` _returnvalue_rotation))
  (bind _asscavenger_character_bp (cast `/Game/TheScavenger/Blueprints/PlayerCharacter/Scavenger_Character_BP` CameraTarget))
  (bind _output_get (set `self.PlayerRef` _asscavenger_character_bp))
  (set `self.FinalCameraRotation` (`Pawn.GetControlRotation` _output_get))
  (set `self.CameraLocation` (+ (`KismetMathLibrary.VLerp` _returnvalue (- _returnvalue_location (* _returnvalue_3 (* (`KismetMathLibrary.Dot_VectorVector` (`KismetMathLibrary.Normal` _returnvalue_2) _returnvalue_3) (/ (`KismetMathLibrary.VSize` _returnvalue_2) 3.0)))) _adscameraalpha) (`KismetMathLibrary.GreaterGreater_VectorRotator` (`self.SwayOffset`) (`self.FinalCameraRotation`))))
  (return (`self.CameraLocation`) (`self.FinalCameraRotation`) (`KismetMathLibrary.Lerp` 90.0 70.0 _adscameraalpha) true))

(fn `UserConstructionScript`)