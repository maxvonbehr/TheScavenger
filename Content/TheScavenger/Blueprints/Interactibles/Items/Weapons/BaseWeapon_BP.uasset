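; Base weapon for the Scavenger player, with stats read from a data table row in the construction script.
; Interaction fires manual, semi-auto or timer-looped automatic shots while held in the primary hand; SwapAction toggles semi/auto.
; Shots play montages and line-trace from the muzzle with accuracy-based random spread, without using the hit result.
; Ammo counters update RoundInChamber; reload selects player magazines by weapon type, with only the assault rifle attaching and animating them.
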(event `StartFire`
  ;[1 1 1] Recoil
)

(event `StopFire`
  ;[1 1 1] Recoil
)

(event `self.Interaction`
  (bind (_weaponstats_weaponid _weaponstats_ammotype _weaponstats_firemode _weaponstats_damage _weaponstats_range _weaponstats_ergonomics _weaponstats_rateoffire _weaponstats_accuracy _weaponstats_reloadmontage _weaponstats_reloademptymontage _weaponstats_manualshootingmontage _weaponstats_shootmontage _weaponstats_playeranimreload _weaponstats_playeranimreloadempty _weaponstats_playeranimcheck _weaponstats_sounddryfire) (break `/Game/TheScavenger/Blueprints/Interactibles/Items/Weapons/WeaponStats` (`self.WeaponStats`)))
  ;[1 1 1] Check if Gun is in Hand
  (if (== (`/Game/TheScavenger/Blueprints/PlayerCharacter/Scavenger_Character_BP.InPrimaryHand` (`self.Player Ref`)) self)
    ;[1 1 1] FireWeapon
    (if (`self.RoundInChamber?`)
      (`self.FireProjectile`)
      (`self.StartFire`)
      (switch `/Game/TheScavenger/Blueprints/Interactibles/Items/Weapons/WeaponFiringModes` (`self.FireMode`)
        (:`NewEnumerator0`
          (bind _returnvalue (`AnimInstance.Montage_Play` (`SkeletalMeshComponent.GetAnimInstance` (`self.WeaponSM`)) _weaponstats_manualshootingmontage 1.0 "MontageLength" 0.0 true))
          (`KismetSystemLibrary.Delay` _returnvalue)
          (if (`self.HasMagazine?`)
            (`self.DecreaseAmmoInMag`)
            (else
              (`self.DecreaseAmmoInternal`)))
          (`self.StopFire`))
        (:`NewEnumerator1`
          (if (`self.HasMagazine?`)
            (`self.DecreaseAmmoInMag`)
            (else
              (`self.DecreaseAmmoInternal`)))
          (`self.StopFire`))
        (:`NewEnumerator2`
          (bind _returnvalue_2 (`KismetSystemLibrary.K2_SetTimerDelegate` (delegate `AutoFire`) (/ 60.0 _weaponstats_rateoffire) true))
          (goto _label :!via `Reset`)))
      (else
        (`GameplayStatics.PlaySound2D` _weaponstats_sounddryfire 1.0 1.0 0.0 null null)))
    (else
      (`KismetSystemLibrary.PrintString` "Hello"))))

(event `AutoFire`
  (bind (_weaponstats_weaponid _weaponstats_ammotype _weaponstats_firemode _weaponstats_damage _weaponstats_range _weaponstats_ergonomics _weaponstats_rateoffire _weaponstats_accuracy _weaponstats_reloadmontage _weaponstats_reloademptymontage _weaponstats_manualshootingmontage _weaponstats_shootmontage _weaponstats_playeranimreload _weaponstats_playeranimreloadempty _weaponstats_playeranimcheck _weaponstats_sounddryfire) (break `/Game/TheScavenger/Blueprints/Interactibles/Items/Weapons/WeaponStats` (`self.WeaponStats`)))
  ;[1 1 1] FireWeapon
  (if (`self.RoundInChamber?`)
    (`self.FireProjectile`)
    (`self.DecreaseAmmoInMag`)
    (else
      (`/Engine/EditorBlueprintResources/StandardMacros.DoOnce` false :!label _label
        (:`Completed`
          (`self.StopFire`)
          (`GameplayStatics.PlaySound2D` _weaponstats_sounddryfire 1.0 1.0 0.0 null null))))))

(event `self.InteractionReleaseInput`
  ;[1 1 1] FireWeapon
  (`KismetSystemLibrary.K2_ClearAndInvalidateTimerHandle` (stale `self.Interaction` _returnvalue_2))
  (`self.StopFire`))

(event `ReloadGun`
  (bind (_weaponstats_weaponid _weaponstats_ammotype _weaponstats_firemode _weaponstats_damage _weaponstats_range _weaponstats_ergonomics _weaponstats_rateoffire _weaponstats_accuracy _weaponstats_reloadmontage _weaponstats_reloademptymontage) (break `/Game/TheScavenger/Blueprints/Interactibles/Items/Weapons/WeaponStats` (`self.WeaponStats`)))
  (bind _weaponstats_weaponid_2 (break `/Game/TheScavenger/Blueprints/Interactibles/Items/Weapons/WeaponStats` (`self.WeaponStats`)))
  (bind (_weaponstats_weaponid_3 _weaponstats_ammotype_2 _weaponstats_firemode_2 _weaponstats_damage_2 _weaponstats_range_2 _weaponstats_ergonomics_2 _weaponstats_rateoffire_2 _weaponstats_accuracy_2 _weaponstats_reloadmontage_2 _weaponstats_reloademptymontage_2 _weaponstats_manualshootingmontage _weaponstats_shootmontage _weaponstats_playeranimreload _weaponstats_playeranimreloadempty) (break `/Game/TheScavenger/Blueprints/Interactibles/Items/Weapons/WeaponStats` (`self.WeaponStats`)))
  (bind _currentmagref (`self.CurrentMagRef`))
  (bind _returnvalue (`SkeletalMeshComponent.GetAnimInstance` (`self.WeaponSM`)))
  (bind _makarovmags (`/Game/TheScavenger/Blueprints/PlayerCharacter/Scavenger_Character_BP.MakarovMags` (`self.Player Ref`)))
  (bind _762magazines (`/Game/TheScavenger/Blueprints/PlayerCharacter/Scavenger_Character_BP.762Magazines` (`self.Player Ref`)))
  (bind _kedrmags (`/Game/TheScavenger/Blueprints/PlayerCharacter/Scavenger_Character_BP.KEDRMags` (`self.Player Ref`)))
  (bind _returnvalue_2 (`KismetArrayLibrary.Array_Length` _kedrmags))
  (bind _returnvalue_3 (`KismetArrayLibrary.Array_Length` _makarovmags))
  (bind _returnvalue_4 (`SkeletalMeshComponent.GetAnimInstance` (`Character.Mesh` (`self.Player Ref`))))
  ;[1 1 1] Reload
  (if (`self.HasExternalMag?`)
    (`/Engine/EditorBlueprintResources/StandardMacros.IsValid` _currentmagref
      (:`Is Valid`
        (if (< (`/Game/TheScavenger/Blueprints/Interactibles/Items/Weapons/BaseGunMagazine.AmmoInClip` _currentmagref) (`/Game/TheScavenger/Blueprints/Interactibles/Items/Weapons/BaseGunMagazine.AmmoMax` _currentmagref))
          (switch `/Game/TheScavenger/Blueprints/Interactibles/Items/Weapons/GameGuns` _weaponstats_weaponid_2 :!label _label_2
            (:`NewEnumerator1`
              (if (> _returnvalue_3 0)
                (set `self.CurrentMagRef` (`|GetArrayItem` _makarovmags (`KismetMathLibrary.RandomIntegerInRange` 0 _returnvalue_3)))))
            (:`NewEnumerator2`
              (if (> _returnvalue_2 0)
                (set `self.CurrentMagRef` (`|GetArrayItem` _kedrmags (`KismetMathLibrary.RandomIntegerInRange` 0 _returnvalue_2)))))
            (:`NewEnumerator4`
              (if (> (`KismetArrayLibrary.Array_Length` _762magazines) 0)
                (bind _output_get (set `self.CurrentMagRef` (`|GetArrayItem` _762magazines)))
                (`KismetArrayLibrary.Array_Remove` _762magazines)
                (`self.SetActorHiddenInGame` _output_get false)
                (`self.K2_AttachToComponent` _output_get (`self.WeaponSM`) "MagSocket" "SnapToTarget" "SnapToTarget" "KeepRelative" true)
                (if (`self.RoundInChamber?`)
                  (`AnimInstance.Montage_Play` _returnvalue _weaponstats_reloadmontage 1.0 "MontageLength" 0.0 true)
                  (`AnimInstance.Montage_Play` _returnvalue_4 _weaponstats_playeranimreload 1.0 "MontageLength" 0.0 true)
                  (else
                    (`AnimInstance.Montage_Play` _returnvalue _weaponstats_reloademptymontage 1.0 "MontageLength" 0.0 true)
                    (`AnimInstance.Montage_Play` _returnvalue_4 _weaponstats_playeranimreloadempty 1.0 "MontageLength" 0.0 true)))
                (set `self.HasMagazine?` true)
                (set `self.RoundInChamber?` true)
                (else
                  (`KismetSystemLibrary.PrintString` "NoAK MAg")))))))
      (:`Is Not Valid`
        (goto _label_2)))))

(event `self.ReceiveBeginPlay`
  (bind (_weaponstats_weaponid _weaponstats_ammotype _weaponstats_firemode) (break `/Game/TheScavenger/Blueprints/Interactibles/Items/Weapons/WeaponStats` (`self.WeaponStats`)))
  ;[1 1 1] GetPlayerRef
  (bind _asscavenger_character_bp (cast `/Game/TheScavenger/Blueprints/PlayerCharacter/Scavenger_Character_BP` (`GameplayStatics.GetPlayerCharacter` 0)))
  (set `self.Player Ref` _asscavenger_character_bp)
  (set `self.FireMode` _weaponstats_firemode))

(event `self.SwapAction`
  ;[1 1 1] Swap
  (`AnimInstance.Montage_Play` (`SkeletalMeshComponent.GetAnimInstance` (`Character.Mesh` (`self.Player Ref`))) "/Game/TheScavenger/Blueprints/PlayerCharacter/AnimMontage/Montage_PlayerAKCheck.Montage_PlayerAKCheck" 1.0 "MontageLength" 0.0 true)
  (`/Engine/EditorBlueprintResources/StandardMacros.FlipFlop`
    (:`A`
      (set `self.FireMode` "NewEnumerator1"))
    (:`B`
      (set `self.FireMode` "NewEnumerator2"))))

(event `LeftTriggerPress`
  (params (PlayerCaller :type "/Game/TheScavenger/Blueprints/PlayerCharacter/Scavenger_Character_BP Object Reference")))

(event `LeftTriggerRelease`
  (params (PlayerCaller :type "/Game/TheScavenger/Blueprints/PlayerCharacter/Scavenger_Character_BP Object Reference")))

(fn `DecreaseAmmoInMag`
  (bind _currentmagref (`self.CurrentMagRef`))
  (bind _ammoinclip (`/Game/TheScavenger/Blueprints/Interactibles/Items/Weapons/BaseGunMagazine.AmmoInClip` _currentmagref))
  (if (> _ammoinclip 0)
    (set `/Game/TheScavenger/Blueprints/Interactibles/Items/Weapons/BaseGunMagazine.AmmoInClip` (- _ammoinclip 1) _currentmagref)
    (set `self.RoundInChamber?` true)
    (else
      (set `/Game/TheScavenger/Blueprints/Interactibles/Items/Weapons/BaseGunMagazine.AmmoInClip` 0 _currentmagref)
      (set `self.RoundInChamber?` false))))

(fn `DecreaseAmmoInternal`
  (if (> (`self.InternalClip`) 0)
    (set `self.InternalClip` (- (`self.InternalClip`) 1))
    (set `self.RoundInChamber?` true)
    (else
      (set `self.InternalClip` 0)
      (set `self.RoundInChamber?` false))))

(fn `FireProjectile`
  (bind _weaponsm (`self.WeaponSM`))
  (bind (_weaponstats_weaponid _weaponstats_ammotype _weaponstats_firemode _weaponstats_damage _weaponstats_range _weaponstats_ergonomics _weaponstats_rateoffire _weaponstats_accuracy _weaponstats_reloadmontage _weaponstats_reloademptymontage _weaponstats_manualshootingmontage _weaponstats_shootmontage) (break `/Game/TheScavenger/Blueprints/Interactibles/Items/Weapons/WeaponStats` (`self.WeaponStats`)))
  (bind (_weaponstats_weaponid_2 _weaponstats_ammotype_2 _weaponstats_firemode_2 _weaponstats_damage_2 _weaponstats_range_2) (break `/Game/TheScavenger/Blueprints/Interactibles/Items/Weapons/WeaponStats` (`self.WeaponStats`)))
  (bind _returnvalue (`SceneComponent.GetSocketLocation` _weaponsm "MuzzleSocket"))
  (`AnimInstance.Montage_Play` (`SkeletalMeshComponent.GetAnimInstance` (`self.WeaponSM`)) _weaponstats_shootmontage 1.0 "MontageLength" 0.0 true)
  (`AnimInstance.Montage_Play` (`SkeletalMeshComponent.GetAnimInstance` (`Character.Mesh` (`self.Player Ref`))) "/Game/TheScavenger/Blueprints/PlayerCharacter/AnimMontage/Montage_PlayerShoot0.Montage_PlayerShoot0" 1.0 "MontageLength" 0.0 true)
  (`KismetSystemLibrary.LineTraceSingle` :`Start` _returnvalue :`End` (+ _returnvalue (* (`self.SpreadTrace` (`KismetMathLibrary.GetForwardVector` (`SceneComponent.GetSocketRotation` _weaponsm "RearSight"))) _weaponstats_range_2)) :`TraceChannel` "TraceTypeQuery1" :`DrawDebugType` "ForDuration"))

(fn `SpreadTrace`
  (params (InputTrace :type "Vector Structure"))
  (returns (SpreadTrace :type "Vector Structure"))
  (bind (_weaponstats_weaponid _weaponstats_ammotype _weaponstats_firemode _weaponstats_damage _weaponstats_range _weaponstats_ergonomics _weaponstats_rateoffire _weaponstats_accuracy) (break `/Game/TheScavenger/Blueprints/Interactibles/Items/Weapons/WeaponStats` (`self.WeaponStats`)))
  (bind _returnvalue (`KismetMathLibrary.MapRangeClamped` _weaponstats_accuracy 0.0 100.0 0.1))
  (bind _returnvalue_2 (* _returnvalue -1.0))
  (return (`KismetMathLibrary.MakeVector` (+ (.x InputTrace) (`KismetMathLibrary.RandomFloatInRange` _returnvalue_2 _returnvalue)) (+ (.y InputTrace) (`KismetMathLibrary.RandomFloatInRange` _returnvalue_2 _returnvalue)) (+ (.z InputTrace) (`KismetMathLibrary.RandomFloatInRange` _returnvalue_2 _returnvalue)))))

(fn `UserConstructionScript`
  (bind _returnvalue (`|GetDataTableRow` "/Game/TheScavenger/Blueprints/Interactibles/Items/Weapons/DataTable_WeaponStats.DataTable_WeaponStats" (`self.Row Name`))
    (:`then`
      (set `self.WeaponStats` _returnvalue)
      (`parent.UserConstructionScript`))))