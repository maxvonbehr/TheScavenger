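; Base melee weapon Blueprint for interactible weapon items, configured from a weapon stats data table.
; The construction script looks up its row by name, stores it as WeaponStats, and runs the parent construction script only when the row is found.
; Interaction is a stub that prints a debug "Hello" when the weapon is not in the player's primary hand.
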(event `self.Interaction`
  ;[1 1 1] Check if Gun is in Hand
  (if (not (== (`/Game/TheScavenger/Blueprints/PlayerCharacter/Scavenger_Character_BP.InPrimaryHand` (`self.Player Ref`)) self))
    (`KismetSystemLibrary.PrintString` "Hello")))

(fn `UserConstructionScript`
  (bind _returnvalue (`|GetDataTableRow` "/Game/TheScavenger/Blueprints/Interactibles/Items/Weapons/DataTable_WeaponStats.DataTable_WeaponStats" (`self.Row Name`))
    (:`then`
      (set `self.WeaponStats` _returnvalue)
      (`parent.UserConstructionScript`))))